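; BP_Camera is a shared camera actor that follows the group of active players once the game starts.
; GameStarted stores the player array and sets a flag that enables the per-tick movement update.
; Each tick, CalculateCameraMovement lerps the Sphere component toward the players' average location by LerpMoveSpeed, a smoothing step that is not scaled by delta time.
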(event EventTick
  (params (DeltaSeconds :type Float%20%28single-precision%29))
  (if (Variables|Default|GetbGameStarted)
    (CallFunction|CalculateCameraMovement)))

(fn ConstructionScript)

(fn GameStarted
  (params (ActivePlayers :type Array%20of%20BP%20Joueur%20Object%20References))
  (Variables|Default|SetActivePlayers ActivePlayers)
  (Variables|Default|SetbGameStarted true))

(fn CalculateCameraMovement
  (Variables|Default|SetPreviousLocation (Transformation|GetWorldLocation (Variables|Default|GetSphere)))
  (bind _returnvalue (Class|GameplayStatics|GetActorArrayAverageLocation (Variables|Default|GetActivePlayers)))
  (Transformation|SetWorldLocation (Variables|Default|GetSphere) (Math|Vector|Lerp(Vector) (Variables|Default|GetPreviousLocation) _returnvalue (Variables|Default|GetLerpMoveSpeed)) false false))