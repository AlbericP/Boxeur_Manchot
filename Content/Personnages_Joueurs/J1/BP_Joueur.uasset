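; BP_Joueur is the shared character for a two-player side-on kicking fighter, with Index selecting material, facing logic and player-specific attack and guard states.
; Input drives X-axis movement, DoOnce-gated mesh flips, jumping, and timed kicks and guards that briefly disable input.
; The kick hitbox overlap launches the opponent away, though only player 1's guard is checked.
; Super attack only prints, and block recoil and sphere trace are unwired.
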(event OnComponentBeginOverlap(Hitbox_Coup)
  (params (OverlappedComponent :type Primitive%20Component%20Object%20Reference) (OtherActor :type Actor%20Object%20Reference) (OtherComp :type Primitive%20Component%20Object%20Reference) (OtherBodyIndex :type Integer) (bFromSweep :type Boolean) (SweepResult :type Hit%20Result%20Structure%20%28by%20ref%29))
  (bind _mesh (Variables|Character|GetMesh))
  (bind _returnvalue (Math|Vector|GetRightVector _mesh))
  (bind _returnvalue_2 (Math|Vector|GetUpVector _mesh))
  (bind _returnvalue_3 (* _returnvalue 4.5e+02))
  (bind _returnvalue_4 (* _returnvalue_2 4.5e+02))
  (bind _returnvalue_5 (+ _returnvalue_3 _returnvalue_4))
  ;[1 1 1] HITBOXS COUPS DE PIEDS
  (bind _asbp_joueur (Utilities|Casting|CastToBP_Joueur OtherActor))
  (if (and (== (Variables|BP_Joueur_C|GetIndex _asbp_joueur) 1) (Variables|Default|GetisAttacking?J1))
    (Development|PrintString "J2 Touché")
    (Character|LaunchCharacter _asbp_joueur _returnvalue_5 true true)
    (elif (Math|Boolean|ANDBoolean (== (Variables|BP_Joueur_C|GetIndex _asbp_joueur) 0) (Variables|Default|GetisAttacking?J2) (not (Variables|Default|GetisGuarding?J1)))
      (Development|PrintString "J1 Touché")
      (Character|LaunchCharacter _asbp_joueur _returnvalue_5 true true))))

(event EventTick
  (params (DeltaSeconds :type Float%20%28single-precision%29))
  ;[1 1 1] TICK
)

(event EventBeginPlay
  ;[1 1 1] Begin play
  (Rendering|Material|SetMaterial (Variables|Character|GetMesh) 0 (Utilities|Select :Index (Variables|Default|GetIndex) :Option%200 "/Game/Materials/MT_Player1Color_Inst.MT_Player1Color_Inst" :Option%201 "/Game/Materials/MT_Player2Colors_Inst.MT_Player2Colors_Inst")))

(event Input|ActionEvents|InputActionStartGame
  (params (Key :type Key%20Structure :default "None"))
  ;[1 1 1] Start Game
  (:Pressed
    (Class|BPIGameMode|StartGame(Message) (Game|GetGameMode))))

(event Input|ActionEvents|InputActionJump
  (params (Key :type Key%20Structure :default "None"))
  (:Pressed
    (Character|Jump)))

(event Input|ActionEvents|InputActionAttack
  (params (Key :type Key%20Structure :default "None"))
  ;[1 0.1134 0.09351] Attack
  (:Pressed
    ;;[1 1 1] j1
    (if (== (Variables|Default|GetIndex) 0)
      ;;[1 1 1] On peut pas frapper si on tombe
      (if (not (AI|Components|NavMovement|IsFalling (Variables|Character|GetCharacterMovement)))
        (if (not (Variables|Default|GetisAttacking?J1))
          (Variables|Default|SetisAttacking?J1 true)
          (Input|DisableInput (Game|GetPlayerController 0))
          (Development|PrintString "Attaque j1")
          (Animation|PlayAnimMontage "/Game/Personnages_Joueurs/Animations/Mma_Kick_Montage.Mma_Kick_Montage" 1.0 "None")
          (Utilities|FlowControl|Delay 0.5)
          (Variables|Default|SetisAttacking?J1 false)
          (Input|EnableInput (Game|GetPlayerController 0))))
      (else
        ;;[1 1 1] On peut pas frapepr si on tombe
        (if (not (AI|Components|NavMovement|IsFalling (Variables|Character|GetCharacterMovement)))
          (if (not (Variables|Default|GetisAttacking?J2))
            (Variables|Default|SetisAttacking?J2 true)
            (Input|DisableInput (Game|GetPlayerController 1))
            (Development|PrintString "Attaque j2")
            (Animation|PlayAnimMontage "/Game/Personnages_Joueurs/Animations/Mma_Kick_Montage.Mma_Kick_Montage" 1.0 "None")
            (Utilities|FlowControl|Delay 0.5)
            (Variables|Default|SetisAttacking?J2 false)
            (Input|EnableInput (Game|GetPlayerController 1))))))))

(event Input|ActionEvents|InputActionSuperAttack
  (params (Key :type Key%20Structure :default "None"))
  ;[1 1 1] Super attack
  (:Pressed
    (if (Variables|Default|GetsuperKickEnabled)
      (Development|PrintString "SUPER ATTACK"))))

(event Input|ActionEvents|InputActionGuard
  (params (Key :type Key%20Structure :default "None"))
  (bind _returnvalue (Game|GetPlayerController 0))
  (bind _returnvalue_2 (Game|GetPlayerController 1))
  ;[1 1 1] Guard
  (:Pressed
    (if (== (Variables|Default|GetIndex) 0)
      (Variables|Default|SetisGuarding?J1 true)
      (Input|DisableInput _returnvalue)
      (Development|PrintString "Guard J1")
      (Utilities|FlowControl|Delay 1.0)
      (Variables|Default|SetisGuarding?J1 false)
      (Input|EnableInput _returnvalue)
      (else
        (Variables|Default|SetisGuarding?J2 true)
        (Input|DisableInput _returnvalue_2)
        (Development|PrintString "Guard J2")
        (Utilities|FlowControl|Delay 0.7)
        (Variables|Default|SetisGuarding?J2 false)
        (Input|EnableInput _returnvalue_2)))))

(event Input|AxisEvents|InputAxisMoveRight
  (params (AxisValue :type Float%20%28single-precision%29))
  (bind _mesh (Variables|Character|GetMesh))
  (bind _mesh_2 (Variables|Character|GetMesh))
  ;[1 1 1] Movement and charatcer rotatino
  (Pawn|Input|AddMovementInput "1.000000, 0, 0" AxisValue false)
  (Utilities|FlowControl|Sequence
    (:then_0
      (if (and (> AxisValue 0.0) (== (Variables|Default|GetIndex) 1))
        (Utilities|FlowControl|DoOnce false :!label _label
          (:Completed
            (Transformation|SetRelativeRotation _mesh_2 "0,90.000000, 0" false false)
            (goto _label_2 Reset)))
        (elif (and (< AxisValue 0.0) (== (Variables|Default|GetIndex) 1))
          (Utilities|FlowControl|DoOnce false :!label _label_2
            (:Completed
              (Transformation|SetRelativeRotation _mesh_2 "0,-90.000000, 0" false false)
              (goto _label Reset))))))
    (:then_1
      (if (and (> AxisValue 0.0) (== (Variables|Default|GetIndex) 0))
        (Utilities|FlowControl|DoOnce false :!label _label_3
          (:Completed
            (Transformation|SetRelativeRotation _mesh "0,-90.000000, 0" false false)
            (goto _label_4 Reset)))
        (elif (and (< AxisValue 0.0) (== (Variables|Default|GetIndex) 0))
          (Utilities|FlowControl|DoOnce false :!label _label_4
            (:Completed
              (Transformation|SetRelativeRotation _mesh "0,90.000000, 0" false false)
              (goto _label_3 Reset))))))))

(fn ConstructionScript)